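; BP_Satelite1 is a spinning satellite that shows a "tweet" message when the ThirdPersonCharacter enters its trigger sphere.
; Tick rotates the Satellite component around yaw at a constant rate.
; Overlap begin slows global time, attaches Tweet1 to the character's capsule and reveals it with a random material from TweetMats.
; Overlap end restores time, hides Tweet1 and reattaches it to the root, with a ReceivingMessage flag guarding both transitions.
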(event OnComponentBeginOverlap(Sphere)
  (params (OverlappedComponent :type Primitive%20Component%20Object%20Reference) (OtherActor :type Actor%20Object%20Reference) (OtherComp :type Primitive%20Component%20Object%20Reference) (OtherBodyIndex :type Integer) (bFromSweep :type Boolean) (SweepResult :type Hit%20Result%20Structure%20%28by%20ref%29))
  (bind _asthird_person_character (Utilities|Casting|CastToThirdPersonCharacter OtherActor))
  (if (not (Variables|Default|GetReceivingMessage))
    (Variables|Default|SetReceivingMessage true)
    (Utilities|Time|SetGlobalTimeDilation 0.2)
    (Transformation|SetWorldLocation (Variables|Default|GetTweet1) (+ "0.000000,50.000000,350.000000" (Transformation|GetWorldLocation (Variables|/Script/Engine.Character|GetCapsuleComponent _asthird_person_character))) false false)
    (Transformation|AttachComponentToComponent (Variables|Default|GetTweet1) (Variables|/Script/Engine.Character|GetCapsuleComponent _asthird_person_character) "None" "SnapToTarget" "KeepWorld" "KeepWorld" true)
    (Transformation|SetRelativeRotation (Variables|Default|GetTweet1) "0.000000,90.000000,90.000000" false false)
    (Rendering|Material|SetMaterial (Variables|Default|GetTweet1) 0 (Utilities|Array|Get(acopy) (Variables|Default|GetTweetMats) (Math|Random|RandomInteger 2)))
    (Development|SetHiddeninGame (Variables|Default|GetTweet1) false false)))

(event OnComponentEndOverlap(Sphere)
  (params (OverlappedComponent :type Primitive%20Component%20Object%20Reference) (OtherActor :type Actor%20Object%20Reference) (OtherComp :type Primitive%20Component%20Object%20Reference) (OtherBodyIndex :type Integer))
  (Utilities|Casting|CastToThirdPersonCharacter OtherActor)
  (if (Variables|Default|GetReceivingMessage)
    (Variables|Default|SetReceivingMessage false)
    (Utilities|Time|SetGlobalTimeDilation 1.0)
    (Development|SetHiddeninGame (Variables|Default|GetTweet1) true false)
    (Transformation|AttachComponentToComponent (Variables|Default|GetTweet1) (Variables|Default|GetDefaultSceneRoot) "None" "KeepRelative" "KeepRelative" "KeepRelative" true)))

(event EventTick
  (params (DeltaSeconds :type Float%20%28single-precision%29))
  (Transformation|AddRelativeRotation (Variables|Default|GetSatellite) (* (Math|Rotator|MakeRotator 0.0 0.0 45.0) DeltaSeconds) false false))

(fn ConstructionScript)