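; BP_LightWay is an actor that kills the player for leaving a fixed corridor along the world Y axis.
; Every Tick it compares player pawn 0's location against hardcoded lower and upper Y bounds, with no trigger volume involved.
; Outside them, it casts the pawn to ThirdPersonCharacter, calls Die, disables input and destroys itself, so it fires only once.
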(event EventTick
  (params (DeltaSeconds :type Float%20%28single-precision%29))
  (bind _returnvalue (Game|Player|GetPlayerPawn 0))
  (bind _returnvalue_2 (Transformation|GetActorLocation _returnvalue))
  (if (or (< (.y _returnvalue_2) (Math|Float|MakeLiteralFloat 5.45e+04)) (> (.y _returnvalue_2) (Math|Float|MakeLiteralFloat 5.54e+04)))
    (bind _asthird_person_character (Utilities|Casting|CastToThirdPersonCharacter (Game|Player|GetPlayerPawn 0)))
    (Default|Die _asthird_person_character false)
    (Input|DisableInput _asthird_person_character (Game|GetPlayerController 0))
    (Actor|DestroyActor)))

(fn ConstructionScript)