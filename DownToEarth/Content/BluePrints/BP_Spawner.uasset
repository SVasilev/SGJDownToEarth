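; BP_Spawner procedurally lays out a vertical field of asteroids, collectable jetpacks and satellites when play begins.
; A single BeginPlay loop starts at the spawner's Z, placing about 200 asteroids and stepping by ZDistance after each.
; Each step may then add a jetpack or, failing that, a satellite, at the next asteroid's height.
; X and Y are randomized within hardcoded world-space bands, and rotations vary by under one degree.
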(event EventBeginPlay
  (Variables|Default|SetCurrentZ (.z (Transformation|GetActorLocation)))
  (for _index (range 0 200)
    (Game|SpawnActorfromClass "/Game/Assets/AsteroidStatic.AsteroidStatic_C" (Math|Transform|MakeTransform (Math|Vector|MakeVector (Math|Random|RandomFloatinRange -6.5e+02 -7.3e+02) (Math|Random|RandomFloatinRange 5.45e+04 5.54e+04) (Variables|Default|GetCurrentZ)) (Math|Rotator|MakeRotator (Math|Random|RandomFloat) (Math|Random|RandomFloat) (Math|Random|RandomFloat))) "Undefined" 0 0)
    (Variables|Default|SetCurrentZ (+ (Variables|Default|GetCurrentZ) (Variables|Default|GetZDistance)))
    ;[1 1 1] 10% Chance to spawn jetpack
    (if (> (Math|Random|RandomFloatinRange 0.0 1e+01) 9.0)
      (Game|SpawnActorfromClass "/Game/BluePrints/CollectableJetpack.CollectableJetpack_C" (Math|Transform|MakeTransform (Math|Vector|MakeVector (Math|Random|RandomFloatinRange -6.5e+02 -7.3e+02) (Math|Random|RandomFloatinRange 5.45e+04 5.54e+04) (Variables|Default|GetCurrentZ)) (Math|Rotator|MakeRotator (Math|Random|RandomFloat) (Math|Random|RandomFloat) (Math|Random|RandomFloat))) "Undefined" 0 0)
      (else
        ;[1 1 1] 20% chance to spawn satelite
        (if (> (Math|Random|RandomFloatinRange 1e+01 2e+01) 18.0)
          (Game|SpawnActorfromClass "/Game/BluePrints/BP_Satelite1.BP_Satelite1_C" (Math|Transform|MakeTransform (Math|Vector|MakeVector (Math|Random|RandomFloatinRange -6.5e+02 -7.3e+02) (Math|Random|RandomFloatinRange 5.45e+04 5.54e+04) (Variables|Default|GetCurrentZ)) (Math|Rotator|MakeRotator (Math|Random|RandomFloat) (Math|Random|RandomFloat) (Math|Random|RandomFloat))) "Undefined" 0 0))))))

(fn ConstructionScript)